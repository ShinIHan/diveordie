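; BP_DiveCharacter is a dive character that shows a main HUD and acts as a dynamic force in the fluid simulation.
; On BeginPlay, if locally controlled, it creates HUD_Main, passes itself to the widget and adds it to the viewport.
; That local-only branch and the Construction Script both find BP_FluidSim_01 and register the character's Mesh as a tracked force component at zero water level.
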(event EventBeginPlay
  (if (Pawn|IsLocallyControlled)
    (bind _returnvalue (UserInterface|CreateWidget "/Game/Blueprints/HUD_Main.HUD_Main_C"))
    (bind _output_get (Variables|Default|SetDiveCharacter_WG _returnvalue))
    (Variables|/Script/game.DiveCharacterWidget|SetCharacter _output_get self)
    (UserInterface|Viewport|AddtoViewport _returnvalue 0)
    (bind _returnvalue_2 (Actor|GetActorOfClass "/Water/FluidSimulation/Blueprints/BP_FluidSim_01.BP_FluidSim_01_C"))
    (Variables|Default|SetSim _returnvalue_2)
    (Utilities|Struct|SetmembersinFluidForceDynamic (Variables|Default|GetFluidForcedDynamic%20Settings) (Variables|Character|GetMesh))
    (Default|RegisterDynamicForce (Variables|Default|GetSim) (Variables|Default|GetFluidForcedDynamic%20Settings) (Variables|Character|GetMesh) 0.0)))

(event Collision|EventActorBeginOverlap
  (params (OtherActor :type Actor%20Object%20Reference)))

(event EventTick
  (params (DeltaSeconds :type Float%20%28single-precision%29)))

(fn ConstructionScript
  (bind _returnvalue (Actor|GetActorOfClass "/Water/FluidSimulation/Blueprints/BP_FluidSim_01.BP_FluidSim_01_C"))
  (Variables|Default|SetSim _returnvalue)
  (Utilities|Struct|SetmembersinFluidForceDynamic (Variables|Default|GetFluidForcedDynamic%20Settings) (Variables|Character|GetMesh))
  (Default|RegisterDynamicForce (Variables|Default|GetSim) (Variables|Default|GetFluidForcedDynamic%20Settings) (Variables|Character|GetMesh) 0.0))