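; BP_InvisibleWall is an invisible-wall actor whose construction script calls Right to spawn another actor of its own class.
; Right places the copy 10000 units along the forward vector with the same rotation, despite its name, so the logic is self-recursive with no stop condition.
; Left mirrors this backward but is never executed.
; The event graph holds only empty default events.
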(event EventBeginPlay)

(event Collision|EventActorBeginOverlap
  (params (OtherActor :type Actor%20Object%20Reference)))

(event EventTick
  (params (DeltaSeconds :type Float%20%28single-precision%29)))

(fn ConstructionScript
  (CallFunction|Right))

(fn Right
  (bind _returnvalue (Transformation|GetActorTransform))
  (Game|SpawnActorfromClass "BP_InvisibleWall_C" (Math|Transform|MakeTransform (+ (* (Transformation|GetActorForwardVector) "10000.000000,10000.000000,10000.000000") (.location _returnvalue)) (.rotation _returnvalue) "1.000000,1.000000,1.000000") "Undefined" 0 0))

(fn Left
  (bind _returnvalue (Transformation|GetActorTransform))
  (Game|SpawnActorfromClass "BP_InvisibleWall_C" (Math|Transform|MakeTransform (+ (* (Transformation|GetActorForwardVector) "-10000.000000,-10000.000000,-10000.000000") (.location _returnvalue)) (.rotation _returnvalue) "1.000000,1.000000,1.000000") "Undefined" 0 0))