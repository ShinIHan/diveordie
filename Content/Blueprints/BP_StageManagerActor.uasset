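; Stage manager actor that carries a location marker widget component for its position in the world.
; Each Tick casts the component's user widget to WGBP_LocationMarker and writes the actor's location into it.
; UpdateDistance only re-caches that widget reference when the cached one is already valid.
; Its distance-in-meters text nodes are unconnected, so no distance is computed or displayed here.
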(event EventBeginPlay)

(event Collision|EventActorBeginOverlap
  (params (OtherActor :type Actor%20Object%20Reference)))

(event EventTick
  (params (DeltaSeconds :type Float%20%28single-precision%29))
  (bind _aswgbp_location_marker (Utilities|Casting|CastToWGBP_LocationMarker (UserInterface|GetUserWidgetObject (Variables|Default|GetMarkerWidget))))
  (Variables|/Game/VFX/WGBP_LocationMarker.WGBP_LocationMarker_C|SetActorLocation _aswgbp_location_marker (Transformation|GetActorLocation)))

(fn ConstructionScript)

(fn UpdateDistance
  (Variables|Default|GetAs%20WGBP%20Location%20Marker
    (:then
      (bind _aswgbp_location_marker (Utilities|Casting|CastToWGBP_LocationMarker (UserInterface|GetUserWidgetObject (Variables|Default|GetMarkerWidget))))
      (Variables|Default|SetAs%20WGBP%20Location%20Marker _aswgbp_location_marker))
    (:else)))